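; Barricade Blueprint whose three static meshes turn into loose physics objects when the interact event fires.
; StartEventonInteract enables physics simulation on the meshes and wakes their rigid bodies.
; After a short delay it sets Hidden In Game to false on them, which leaves them visible rather than hiding them.
; The construction script only calls the parent's.
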(event `self.StartEventOnInteract`
  (bind _staticmesh (`self.StaticMesh`))
  (`PrimitiveComponent.SetSimulatePhysics` _staticmesh true)
  (`PrimitiveComponent.SetSimulatePhysics` (`self.StaticMesh1`) true)
  (`PrimitiveComponent.SetSimulatePhysics` (`self.StaticMesh2`) true)
  (`PrimitiveComponent.WakeAllRigidBodies` _staticmesh)
  (`PrimitiveComponent.WakeAllRigidBodies` (`self.StaticMesh1`))
  (`PrimitiveComponent.WakeAllRigidBodies` (`self.StaticMesh2`))
  (`KismetSystemLibrary.Delay` 2.0)
  (`SceneComponent.SetHiddenInGame` (`self.StaticMesh`) false false)
  (`SceneComponent.SetHiddenInGame` (`self.StaticMesh1`) false false)
  (`SceneComponent.SetHiddenInGame` (`self.StaticMesh2`) false false))

(fn `UserConstructionScript`
  (`parent.UserConstructionScript`))