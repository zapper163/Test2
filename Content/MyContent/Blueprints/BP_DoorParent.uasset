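; Parent door Blueprint that swings open on a hinge and shows a text label when something enters its interaction radius.
; OpenDoor, not called within this graph, plays a timeline that lerps the door's relative yaw, then sets IsOpen.
; Radius overlaps show and hide the text only while IsOpen is false; finishing the opening also unhides it, so later overlaps leave it visible.
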(event `Open Door`
  ;[1 1 1] Comment
  (bind (_direction _dooralpha) (`Timeline|DoorAnimation`)
    (:`Update`
      (`SceneComponent.K2_SetRelativeRotation` (`self.Door`) (`KismetMathLibrary.RLerp` (struct) (struct :`Yaw` -110.0) _dooralpha true) false false))
    (:`Finished`
      (set `self.isOpen` true)
      (`SceneComponent.SetHiddenInGame` (`self.TextRender`) false false))))

(event `self.InteractiveRadius.OnComponentBeginOverlap`
  (params (OverlappedComponent :type "PrimitiveComponent Object Reference") (OtherActor :type "Actor Object Reference") (OtherComp :type "PrimitiveComponent Object Reference") (OtherBodyIndex :type Integer) (bFromSweep :type Boolean) (SweepResult :type "HitResult Structure (by ref)"))
  (if (not (`self.isOpen`))
    (`SceneComponent.SetHiddenInGame` (`self.TextRender`) false false)))

(event `self.InteractiveRadius.OnComponentEndOverlap`
  (params (OverlappedComponent :type "PrimitiveComponent Object Reference") (OtherActor :type "Actor Object Reference") (OtherComp :type "PrimitiveComponent Object Reference") (OtherBodyIndex :type Integer))
  (if (not (`self.isOpen`))
    (`SceneComponent.SetHiddenInGame` (`self.TextRender`) true false)))

(fn `UserConstructionScript`)