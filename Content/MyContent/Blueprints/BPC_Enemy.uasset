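; Patrolling enemy actor that moves along a referenced path's spline and signals when the player character type enters its vision cone.
; A timeline scaled by SecondsToCompletePath drives location and rotation along the spline from BeginPlay, and StopDelay pauses it for a given time.
; Cone overlaps with the ALS AnimMan character switch the spotlight between altered and unseen colors.
; Interact unhides the actor.
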(event `self.ReceiveBeginPlay`
  (`self.MoveEnemy`))

(event `/Game/MyContent/Interfaces/BPI_Interaction.Interact`
  (`self.SetActorHiddenInGame` false))

(event `StopDelay`
  (params (delay :type "Float (double-precision)"))
  (`TimelineComponent.Stop` (`self.Timeline`))
  (`KismetSystemLibrary.Delay` delay)
  (`TimelineComponent.Play` (`self.Timeline`)))

(event `MoveEnemy`
  (`TimelineComponent.SetPlayRate` (`self.Timeline`) (/ 1.0 (`self.SecondsToCompletePath`)))
  (bind (_direction _newtrack_0) (`Timeline|Timeline`)
    (:`Update`
      (bind _returnvalue (`KismetMathLibrary.Lerp` 0.0 (`SplineComponent.GetSplineLength` (`/Game/MyContent/Blueprints/BP_Spline.Spline` (`self.Path`))) _newtrack_0))
      (`self.K2_SetActorTransform` (`KismetMathLibrary.MakeTransform` (`SplineComponent.GetLocationAtDistanceAlongSpline` (`/Game/MyContent/Blueprints/BP_Spline.Spline` (`self.Path`)) _returnvalue "World") (`SplineComponent.GetRotationAtDistanceAlongSpline` (`/Game/MyContent/Blueprints/BP_Spline.Spline` (`self.Path`)) _returnvalue "Local"))))))

(event `self.Cone.OnComponentBeginOverlap`
  (params (OverlappedComponent :type "PrimitiveComponent Object Reference") (OtherActor :type "Actor Object Reference") (OtherComp :type "PrimitiveComponent Object Reference") (OtherBodyIndex :type Integer) (bFromSweep :type Boolean) (SweepResult :type "HitResult Structure (by ref)"))
  (cast `/Game/AdvancedLocomotionV4/Blueprints/CharacterLogic/ALS_AnimMan_CharacterBP` OtherActor)
  (`LightComponent.SetLightColor` (`self.SpotLight`) (`self.alteredColor`) true))

(event `self.Cone.OnComponentEndOverlap`
  (params (OverlappedComponent :type "PrimitiveComponent Object Reference") (OtherActor :type "Actor Object Reference") (OtherComp :type "PrimitiveComponent Object Reference") (OtherBodyIndex :type Integer))
  (cast `/Game/AdvancedLocomotionV4/Blueprints/CharacterLogic/ALS_AnimMan_CharacterBP` OtherActor)
  (`LightComponent.SetLightColor` (`self.SpotLight`) (`self.unseenColor`) true))

(fn `UserConstructionScript`
  (`parent.UserConstructionScript`))