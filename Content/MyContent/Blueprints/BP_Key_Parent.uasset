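; BP_Key_Parent is a base key pickup that unlocks a list of linked actors when the player interacts with it.
; A one-time Interact marks it taken, hides the mesh and prompt, disables collision, and sends UnlockMessage to ActorToUnlock entries implementing BPI_Interaction.
; It then calls StartEventOnTaken, an empty hook.
; InteractionRadius overlaps show the text prompt until taken, though end overlap also shows it rather than hiding it.
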(event `/Game/MyContent/Interfaces/BPI_Interaction.Interact`
  (`/Engine/EditorBlueprintResources/StandardMacros.DoOnce` false
    (:`Completed`
      (set `self.isTaken` true)
      (`SceneComponent.SetHiddenInGame` (`self.StaticMesh`) true false)
      (`SceneComponent.SetHiddenInGame` (`self.TextRender_UI`) true false)
      (`self.SetActorEnableCollision` self false)
      (for _array_element (`self.ActorToUnlock`)
        (if (`KismetSystemLibrary.DoesImplementInterface` _array_element "/Game/MyContent/Interfaces/BPI_Interaction.BPI_Interaction_C")
          (message `/Game/MyContent/Interfaces/BPI_Interaction.Unlock` _array_element)))
      (`self.StartEventOnTaken`))))

(event `StartEventOnTaken`)

(event `self.InteractionRadius.OnComponentBeginOverlap`
  (params (OverlappedComponent :type "PrimitiveComponent Object Reference") (OtherActor :type "Actor Object Reference") (OtherComp :type "PrimitiveComponent Object Reference") (OtherBodyIndex :type Integer) (bFromSweep :type Boolean) (SweepResult :type "HitResult Structure (by ref)"))
  (if (not (`self.isTaken`))
    (`SceneComponent.SetHiddenInGame` (`self.TextRender_UI`) false false)))

(event `self.InteractionRadius.OnComponentEndOverlap`
  (params (OverlappedComponent :type "PrimitiveComponent Object Reference") (OtherActor :type "Actor Object Reference") (OtherComp :type "PrimitiveComponent Object Reference") (OtherBodyIndex :type Integer))
  (if (not (`self.isTaken`))
    (`SceneComponent.SetHiddenInGame` (`self.TextRender_UI`) false false)))

(fn `UserConstructionScript`)