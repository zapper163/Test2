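; BPC_Switch is an interactable switch built on a parent Blueprint that depresses its button mesh when used.
; On interact, a locked switch shows its locked text through InteractUI; otherwise a DoOnce lets a timeline lower the mesh a single time, then calls OnInteractionComplete when finished.
; The construction script colors the mesh by lock state, using a red grid material when locked.
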(event `self.StartEventOnInteract`
  (if (`self.isLocked`)
    (`TextRenderComponent.K2_SetText` (`self.InteractUI`) (`self.LockedText`))
    (else
      (`/Engine/EditorBlueprintResources/StandardMacros.DoOnce` false
        (:`Completed`
          (bind (_direction _button) (`Timeline|Timeline`)
            (:`Update`
              (`SceneComponent.K2_SetRelativeLocation` (`self.StaticMesh`) (`KismetMathLibrary.VLerp` (0.0 0.0 0.0) (0.0 0.0 -5.0) _button) false false))
            (:`Finished`
              (`self.OnInteractionComplete`))))))))

(fn `UserConstructionScript`
  (`parent.UserConstructionScript`)
  (if (`self.isLocked`)
    (`PrimitiveComponent.SetMaterial` (`self.StaticMesh`) 0 "/Game/Materials/M_LDGrid_Red.M_LDGrid_Red")
    (else
      (`PrimitiveComponent.SetMaterial` (`self.StaticMesh`) 0 "/Game/AdvancedLocomotionV4/Environment/Materials/M_Landscape.M_Landscape"))))