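; Lockable door actor that responds to Interact and Unlock events.
; Interact shows the locked message on its TextRender while locked; otherwise a DoOnce calls OpenDoor a single time and sets the text visible in game.
; Unlock clears the IsLocked flag and switches the text to the unlocked message, without opening the door.
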(event `/Game/MyContent/Interfaces/BPI_Interaction.Interact`
  (if (`self.isLocked`)
    (`TextRenderComponent.K2_SetText` (`self.TextRender`) (`self.LockedText`))
    (else
      (`/Engine/EditorBlueprintResources/StandardMacros.DoOnce` false
        (:`Completed`
          (`self.Open Door`)
          (`SceneComponent.SetHiddenInGame` (`self.TextRender`) false false))))))

(event `/Game/MyContent/Interfaces/BPI_Interaction.Unlock`
  (set `self.isLocked` false)
  (`TextRenderComponent.K2_SetText` (`self.TextRender`) (`self.UnlockedText`)))

(fn `UserConstructionScript`
  (`parent.UserConstructionScript`))