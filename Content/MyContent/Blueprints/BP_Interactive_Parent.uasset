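; Base Blueprint for one-time interactable objects that can start locked, with child Blueprints overriding StartEventOnInteract for their own behavior.
; InteractionRadius overlaps show the InteractUI prompt until interaction completes and hide it on exit.
; Interact shows locked text when locked; otherwise it marks completion, hides radius and prompt, and calls the child hook.
; Unlock clears the lock and swaps in the unlocked text.
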(event `/Game/MyContent/Interfaces/BPI_Interaction.Interact`
  (if (`self.isLocked`)
    (`TextRenderComponent.K2_SetText` (`self.InteractUI`) (`self.LockedText`))
    (else
      (set `self.InteractComplete` true)
      (`SceneComponent.SetHiddenInGame` (`self.InteractionRadius`) true false)
      (`SceneComponent.SetHiddenInGame` (`self.InteractUI`) true false)
      (`self.StartEventOnInteract`))))

(event `StartEventOnInteract`)

(event `/Game/MyContent/Interfaces/BPI_Interaction.Unlock`
  (set `self.isLocked` false)
  (`TextRenderComponent.K2_SetText` (`self.InteractUI`) (`self.UnlockedText`)))

(event `self.InteractionRadius.OnComponentBeginOverlap`
  (params (OverlappedComponent :type "PrimitiveComponent Object Reference") (OtherActor :type "Actor Object Reference") (OtherComp :type "PrimitiveComponent Object Reference") (OtherBodyIndex :type Integer) (bFromSweep :type Boolean) (SweepResult :type "HitResult Structure (by ref)"))
  (if (not (`self.InteractComplete`))
    (`SceneComponent.SetHiddenInGame` (`self.InteractUI`) false false)))

(event `self.InteractionRadius.OnComponentEndOverlap`
  (params (OverlappedComponent :type "PrimitiveComponent Object Reference") (OtherActor :type "Actor Object Reference") (OtherComp :type "PrimitiveComponent Object Reference") (OtherBodyIndex :type Integer))
  (if (not false)
    (`SceneComponent.SetHiddenInGame` (`self.InteractUI`) true false)))

(fn `UserConstructionScript`)